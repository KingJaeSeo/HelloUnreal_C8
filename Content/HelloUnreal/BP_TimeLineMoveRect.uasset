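; Actor Blueprint that moves its Sphere component endlessly around a square path in the local X-Z plane, starting at BeginPlay.
; One Timeline drives all four sides, playing forward for Right and Up and in reverse for Left and Down.
; UpdateMove scales the Timeline value by EndPoint to set the active axis.
; On finish, ChangeMoveType advances the MoveType state and execution loops back to play the next side.
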(event `self.ReceiveBeginPlay`
  ;[1 1 1] 상태에 따른 실행라인 방향 처리
  (switch `/Game/HelloUnreal/En_MoveType` (`self.MoveType`) :!label _label
    (:`NewEnumerator0`
      (bind (_direction _value) (`Timeline|타임라인_0` :`NewTime` 2.5 :!via `PlayFromStart` :!label _label_2)
        (:`Update`
          (`self.UpdateMove` _value))
        (:`Finished`
          (`self.ChangeMoveType`)
          (goto _label))))
    (:`NewEnumerator1`
      (goto _label_2 :!via `PlayFromStart`))
    (:`NewEnumerator2`
      (goto _label_2 :!via `ReverseFromEnd`))
    (:`NewEnumerator3`
      (goto _label_2 :!via `ReverseFromEnd`))))

(fn `ChangeMoveType`
  ;[1 1 1] 방향 바꾸기
  (switch `/Game/HelloUnreal/En_MoveType` (`self.MoveType`)
    (:`NewEnumerator0`
      (set `self.MoveType` "NewEnumerator1"))
    (:`NewEnumerator1`
      (set `self.MoveType` "NewEnumerator2"))
    (:`NewEnumerator2`
      (set `self.MoveType` "NewEnumerator3"))
    (:`NewEnumerator3`
      (set `self.MoveType` "NewEnumerator0"))))

(fn `UpdateMove`
  (params (Value :type "Float (double-precision)"))
  (bind _sphere (`self.Sphere`))
  (bind _sphere_2 (`self.Sphere`))
  (bind _returnvalue (* Value (`self.EndPoint`)))
  (bind (_relativelocation_x _relativelocation_y) (`KismetMathLibrary.BreakVector` (`SceneComponent.RelativeLocation` _sphere)))
  (bind (_relativelocation_x_2 _relativelocation_y_2 _relativelocation_z) (`KismetMathLibrary.BreakVector` (`SceneComponent.RelativeLocation` _sphere_2)))
  (switch `/Game/HelloUnreal/En_MoveType` (`self.MoveType`)
    (:`NewEnumerator0`
      (`SceneComponent.K2_SetRelativeLocation` _sphere_2 (`KismetMathLibrary.MakeVector` _returnvalue _relativelocation_y_2 _relativelocation_z) false false :!label _label))
    (:`NewEnumerator1`
      (`SceneComponent.K2_SetRelativeLocation` _sphere (`KismetMathLibrary.MakeVector` _relativelocation_x _relativelocation_y _returnvalue) false false :!label _label_2))
    (:`NewEnumerator2`
      (goto _label))
    (:`NewEnumerator3`
      (goto _label_2))))

(fn `UserConstructionScript`)